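; Enemy character Blueprint that detects targets ahead, triggers its attack animation and fires hitscan guns.
; BeginPlay loads the selected weapon class and socket-attaches it, dual-wielded for Pistol and Uzi.
; A per-tick forward box trace stores hit distance and sets IsAttack on the AnimBP; turn-to-target logic is unconnected.
; Left/right fire events range-check, activate guns and line-trace damage; incoming damage only lowers and prints Health.
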(event Custom|FireActivateRight
  (bind _rightgunbase (Variables|Default|GetrightGunBase))
  (bind _output (Utilities|ResolveSoftReference _rightgunbase))
  ;[1 1 1] FireEvent
  (if (< (Variables|Default|GetDistance) 1.5e+03)
    (Default|WeaponActivate _output)
    (CallFunction|FireDamageAttack _output)))

(event Custom|FireActivateLeft
  (bind _leftgunbase (Variables|Default|GetleftGunBase))
  (bind _output (Utilities|ResolveSoftReference _leftgunbase))
  ;[1 1 1] FireEvent
  (if (< (Variables|Default|GetDistance) 1.5e+03)
    (Default|WeaponActivate _output)
    (CallFunction|FireDamageAttack _output)))

(event Game|Damage|EventAnyDamage
  (params (Damage :type Float%20%28single-precision%29) (DamageType :type Damage%20Type%20Object%20Reference) (InstigatedBy :type Controller%20Object%20Reference) (DamageCauser :type Actor%20Object%20Reference))
  ;[1 1 1] Receive Damage
  (bind _output_get (Variables|Default|SetHealth (- (Variables|Default|GetHealth) Damage)))
  (Development|PrintString (Utilities|String|ToString(Float) _output_get)))

(event EventTick
  (params (DeltaSeconds :type Float%20%28single-precision%29))
  ;[1 1 1] Event Tick
  (Utilities|FlowControl|Sequence
    (:then_0
      (CallFunction|FindSoldier))))

(event EventBeginPlay
  ;[1 1 1] BeginPlay
  (CallFunction|WeaponSpawn))

(fn ConstructionScript)

(fn FireDamageAttack
  (params (WeaponTarget :type Base%20Gun%20Bp%20Object%20Reference))
  (bind _gunstaticmesh (Variables|/Game/Guns/Gun_Bp/BaseGun_Bp.BaseGun_Bp_C|GetGunStaticMesh WeaponTarget))
  (bind _returnvalue (Transformation|GetSocketLocation _gunstaticmesh "Muzzle"))
  (bind _outhit (Collision|LineTraceByChannel _returnvalue (+ _returnvalue (* (Math|Vector|GetForwardVector (Transformation|GetWorldRotation (Variables|Default|GetDefaultSceneRoot))) 1e+03)) "TraceTypeQuery3" false 0 "ForDuration"))
  (Game|Damage|ApplyDamage (.HitActor (Collision|BreakHitResult _outhit)) (Variables|Default|GetdamageCount) 0 0))

(fn SetAttackAnim
  (bind _asenemy_anim_bp (Utilities|Casting|CastToEnemyAnimBp (Components|SkeletalMesh|GetAnimInstance (Variables|Default|GetEnemy))))
  (Variables|/Game/Character/Blueprint/enemy/EnemyAnimBp.EnemyAnimBp_C|SetisAttack _asenemy_anim_bp true))

(fn WeaponAttach
  (params (Class :type Actor%20Class%20Reference) (InSocketName :type Name))
  (bind _enemy (Variables|Default|GetEnemy))
  (bind _returnvalue (Game|SpawnActorfromClass Class (Transformation|GetSocketTransform _enemy InSocketName "RTS_World") "Undefined" 0 0))
  (bind _asbase_gun_bp (Utilities|Casting|CastToBaseGun_Bp _returnvalue))
  (Transformation|AttachComponentToComponent _returnvalue _enemy InSocketName "SnapToTarget" "SnapToTarget" "SnapToTarget" true)
  (return _asbase_gun_bp))

(fn WeaponSpawn
  (bind _enemyanimselector (Variables|Default|GetenemyAnimSelector))
  (bind _returnvalue (Utilities|LoadClassAssetBlocking (Utilities|Array|Get(acopy) (Variables|Default|GetWeapons) (Math|Conversions|ToInteger(Byte) _enemyanimselector))))
  (bind _asactor (Utilities|Casting|CastToActorClass _returnvalue))
  (switch Utilities|FlowControl|Switch|SwitchonEnemyAnimSelector _enemyanimselector
    (:NewEnumerator0
      (bind _asbase_gun_bp (CallFunction|WeaponAttach _asactor "RightWeaponSocket" :!label _label))
      (Variables|Default|SetrightGunBase (Utilities|ResolveSoftReference _asbase_gun_bp))
      (bind _asbase_gun_bp_2 (CallFunction|WeaponAttach _asactor "LeftWeaponSocket"))
      (Variables|Default|SetleftGunBase (Utilities|ResolveSoftReference _asbase_gun_bp_2)))
    (:NewEnumerator1
      (goto _label))
    (:NewEnumerator2
      (bind _asbase_gun_bp_3 (CallFunction|WeaponAttach _asactor "RightWeaponSocket" :!label _label_2))
      (Variables|Default|SetrightGunBase (Utilities|ResolveSoftReference _asbase_gun_bp_3)))
    (:NewEnumerator3
      (goto _label_2))
    (:NewEnumerator4
      (goto _label_2))
    (:NewEnumerator5
      (goto _label_2)))
  (|SetBy-RefVar _asactor))

(event Custom|FindSoldier
  (bind _returnvalue (Transformation|GetActorLocation))
  (bind (_outhit _returnvalue_2) (Collision|BoxTraceByChannel _returnvalue (+ _returnvalue (* (Transformation|GetActorForwardVector) 2e+03)) "300.000000,300.000000,50.000000" "0,0.000000,0.000000" "TraceTypeQuery3" false 0 "ForDuration" true "(R=1.000000,G=0.000000,B=0.000000,A=1.000000)" "(R=0.000000,G=1.000000,B=0.000000,A=1.000000)" 0.1))
  (if _returnvalue_2
    (Utilities|IsValid (.HitActor (Collision|BreakHitResult _outhit))
      (:Is%20Valid
        (Variables|Default|SetDistance (.Distance (Collision|BreakHitResult _outhit)))
        (CallFunction|SetAttackAnim)))))