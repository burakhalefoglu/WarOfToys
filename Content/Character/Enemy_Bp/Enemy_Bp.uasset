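; Armed enemy that detects targets, turns to face them and attacks with the weapon chosen by its anim selector.
; BeginPlay loads the gun class and socket-attaches it, one per hand for Pistol and Uzi, otherwise right only.
; A per-tick box trace stores target distance, snaps rotation, then sets the AnimInstance attack flag.
; Left/right fire events activate guns within range and apply line-trace damage; incoming damage only lowers and prints health.
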(event Custom|FireActivateRight
  (bind _rightgunbase (Variables|Default|GetRightGunBase))
  ;[1 1 1] FireEvent
  (if (< (Variables|Default|GetDistance) 1.5e+03)
    (Default|WeaponActivate _rightgunbase)
    (CallFunction|FireDamageAttack _rightgunbase)))

(event Custom|FireActivateLeft
  (bind _leftgunbase (Variables|Default|GetLeftGunBase))
  ;[1 1 1] FireEvent
  (if (< (Variables|Default|GetDistance) 1.5e+03)
    (Default|WeaponActivate _leftgunbase)
    (CallFunction|FireDamageAttack _leftgunbase)))

(event Game|Damage|EventAnyDamage
  (params (Damage :type Float%20%28single-precision%29) (DamageType :type Damage%20Type%20Object%20Reference) (InstigatedBy :type Controller%20Object%20Reference) (DamageCauser :type Actor%20Object%20Reference))
  ;[1 1 1] Receive Damage
  (bind _output_get (Variables|Default|SetHealht (- (Variables|Default|GetHealht) Damage)))
  (Development|PrintString (Utilities|String|ToString(Float) _output_get)))

(event EventTick
  (params (DeltaSeconds :type Float%20%28single-precision%29))
  ;[1 1 1] Event Tick
  (Utilities|FlowControl|Sequence
    (:then_0
      (CallFunction|FindSoldier))))

(event EventBeginPlay
  ;[1 1 1] BeginPlay
  (CallFunction|WeaponSpawn))

(fn ConstructionScript)

(fn WeaponSpawn
  (bind _enemyanimselector (Variables|Default|GetEnemyAnimSelector))
  (bind _returnvalue (Utilities|LoadClassAssetBlocking (Utilities|Array|Get(acopy) (Variables|Default|GetWeapons) (Math|Conversions|ToInteger(Byte) _enemyanimselector))))
  (bind _asactor (Utilities|Casting|CastToActorClass _returnvalue))
  (switch Utilities|FlowControl|Switch|SwitchonEnemyAnimSelector _enemyanimselector
    (:NewEnumerator0
      (bind _asgun_base_bp (CallFunction|WeaponAttach "RightWeaponSocket" _asactor :!label _label))
      (Variables|Default|SetRightGunBase _asgun_base_bp)
      (bind _asgun_base_bp_2 (CallFunction|WeaponAttach "LeftWeaponSocket" _asactor))
      (Variables|Default|SetLeftGunBase _asgun_base_bp_2))
    (:NewEnumerator1
      (goto _label))
    (:NewEnumerator2
      (bind _asgun_base_bp_3 (CallFunction|WeaponAttach "RightWeaponSocket" _asactor :!label _label_2))
      (Variables|Default|SetRightGunBase _asgun_base_bp_3))
    (:NewEnumerator3
      (goto _label_2))
    (:NewEnumerator4
      (goto _label_2))
    (:NewEnumerator5
      (goto _label_2)))
  (|SetBy-RefVar _asactor))

(fn WeaponAttach
  (params (InSocketName :type Name) (Class :type Actor%20Class%20Reference))
  (bind _enemy (Variables|Default|GetEnemy))
  (bind _returnvalue (Game|SpawnActorfromClass Class (Transformation|GetSocketTransform _enemy InSocketName "RTS_World") "Undefined" 0 0))
  (bind _asgun_base_bp (Utilities|Casting|CastToGunBase_Bp _returnvalue))
  (Transformation|AttachComponentToComponent _returnvalue _enemy InSocketName "SnapToTarget" "SnapToTarget" "SnapToTarget" true)
  (return _asgun_base_bp))

(fn SetAttackAnim
  (bind _asenemy_with_weapon (Utilities|Casting|CastToEnemyWithWeapon (Components|SkeletalMesh|GetAnimInstance (Variables|Default|GetEnemy))))
  (Variables|/Game/Character/Enemy_Bp/EnemyWithWeapon.EnemyWithWeapon_C|SetİsAttack? _asenemy_with_weapon true))

(fn FireDamageAttack
  (params (WeaponTarget :type Gun%20Base%20Bp%20Object%20Reference))
  (bind _gunstaticmesh (Variables|/Game/Guns/Blueprints/GunBase_Bp.GunBase_Bp_C|GetGunStaticMesh WeaponTarget))
  (bind _returnvalue (Transformation|GetSocketLocation _gunstaticmesh "Muzzle"))
  (bind _outhit (Collision|LineTraceByChannel _returnvalue (+ _returnvalue (* (Math|Vector|GetForwardVector (Transformation|GetWorldRotation (Variables|Default|GetDefaultSceneRoot))) 1e+03)) "TraceTypeQuery3" false 0 "ForDuration"))
  (Game|Damage|ApplyDamage (.HitActor (Collision|BreakHitResult _outhit)) (Variables|Default|GetDamageCount) 0 0))

(event Custom|FindSoldier
  (bind _returnvalue (Transformation|GetActorLocation))
  (bind (_outhit _returnvalue_2) (Collision|BoxTraceByChannel (Math|Vector|MakeVector (.x _returnvalue) (.y _returnvalue) (.z _returnvalue)) (Math|Vector|MakeVector (* (.x _returnvalue) 5.0) (.y _returnvalue) (.z _returnvalue)) "50.000000,1000.000000,100.000000" "0, 0, 0" "TraceTypeQuery3" false 0 "ForDuration" true "(R=1.000000,G=0.000000,B=0.000000,A=1.000000)" "(R=0.000000,G=1.000000,B=0.000000,A=1.000000)" 0.1))
  (if _returnvalue_2
    (Utilities|IsValid (.HitActor (Collision|BreakHitResult _outhit))
      (:Is%20Valid
        (Variables|Default|SetDistance (.Distance (Collision|BreakHitResult _outhit)))
        (if (Math|Rotator|Equal(Rotator) (Transformation|GetWorldRotation (Variables|Default|GetCapsule)) (Math|Rotator|FindLookatRotation (Transformation|GetWorldLocation (Variables|Default|GetCapsule)) (Transformation|GetWorldLocation (.HitComponent (Collision|BreakHitResult _outhit)))) 0.0001)
          (CallFunction|SetAttackAnim)
          (else
            (Transformation|SetActorRotation (Math|Rotator|FindLookatRotation (Transformation|GetWorldLocation (Variables|Default|GetCapsule)) (Transformation|GetWorldLocation (.HitComponent (Collision|BreakHitResult _outhit)))))))))))